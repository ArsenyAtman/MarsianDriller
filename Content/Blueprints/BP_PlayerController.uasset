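; Player controller that drives the possessed BP_Rover from input.
; Movement axes push the rover relative to its CineCamera, using the camera's forward and right vectors flattened onto the ground plane and normalized.
; The Interact action forwards to the rover's Interact function.
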(event `InputAxis|MoveUpDown`
  (params (AxisValue :type "Float (single-precision)"))
  (`Pawn.AddMovementInput` (`self.GetRover`) (* AxisValue (`self.GetAbsoluteForward`)) 1.0 false))

(event `InputAxis|MoveRigthLeft`
  (params (AxisValue :type "Float (single-precision)"))
  (`Pawn.AddMovementInput` (`self.GetRover`) (* AxisValue (`self.GetAbsoluteRight`)) 1.0 false))

(event `InputAction|Interact`
  (params (Key :type "Key Structure"))
  (:`Pressed`
    (`/Game/Blueprints/BP_Rover.Interact` (`self.GetRover`))))

(fn `GetAbsoluteForward`
  (returns (AbsoluteForward :type "Vector Structure"))
  (return (`KismetMathLibrary.Normal` (`KismetMathLibrary.ProjectVectorOnToPlane` (`SceneComponent.GetForwardVector` (`/Game/Blueprints/BP_Rover.CineCamera` (`self.GetRover`))) (0.0 0.0 1.0)))))

(fn `GetAbsoluteRight`
  (returns (AbsoluteRigth :type "Vector Structure"))
  (return (`KismetMathLibrary.Normal` (`KismetMathLibrary.ProjectVectorOnToPlane` (`SceneComponent.GetRightVector` (`/Game/Blueprints/BP_Rover.CineCamera` (`self.GetRover`))) (0.0 0.0 1.0)))))

(fn `GetRover`
  (returns (Rover :type "/Game/Blueprints/BP_Rover Object Reference"))
  (return (cast `/Game/Blueprints/BP_Rover` (`self.K2_GetPawn`) :!pure true)))

(fn `UserConstructionScript`)