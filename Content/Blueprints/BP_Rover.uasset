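; BP_Rover is a rover actor that carries two BP_Storage tanks as child actors, zeroed on BeginPlay.
; Interact line-traces forward from an arrow, sends InteractMessage with itself to the hit actor, and briefly shows a cylinder.
; FillTanks adds the given amount to each tank.
; EmptyTanks zeroes both but returns only the first tank's previous volume.
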(event `self.ReceiveBeginPlay`
  (bind _asbp_storage (cast `/Game/Blueprints/BP_Storage` (`ChildActorComponent.ChildActor` (`self.ChildActor`))))
  (set `self.Storage1` _asbp_storage)
  (bind _asbp_storage_2 (cast `/Game/Blueprints/BP_Storage` (`ChildActorComponent.ChildActor` (`self.ChildActor1`))))
  (set `self.Storage2` _asbp_storage_2)
  (`/Game/Blueprints/BP_Storage.UpdateValue` (`self.Storage1`) 0.0)
  (`/Game/Blueprints/BP_Storage.UpdateValue` (`self.Storage2`) 0.0))

(event `Interact`
  (bind _arrow1 (`self.Arrow1`))
  (bind _returnvalue (`SceneComponent.K2_GetComponentLocation` _arrow1))
  (bind _outhit (`KismetSystemLibrary.LineTraceSingleForObjects` _returnvalue (+ _returnvalue (* (`self.TraceLength`) (`SceneComponent.GetForwardVector` _arrow1))) (`|MakeArray` "ObjectTypeQuery1" "ObjectTypeQuery2" :!type "EObjectTypeQuery Enum")))
  (message `/Game/Blueprints/BPI_Interactable.Interact` (`.HitActor` (`GameplayStatics.BreakHitResult` _outhit)) self)
  (`SceneComponent.SetVisibility` (`self.Cylinder`) true true)
  (`KismetSystemLibrary.Delay` 0.2)
  (`SceneComponent.SetVisibility` (`self.Cylinder`) false true))

(event `FillTanks`
  (params (ValueToAdd :type "Float (double-precision)"))
  (bind _storage1 (`self.Storage1`))
  (bind _storage2 (`self.Storage2`))
  (`/Game/Blueprints/BP_Storage.UpdateValue` _storage1 (+ ValueToAdd (`/Game/Blueprints/BP_Storage.CurrentVolume` _storage1)))
  (`/Game/Blueprints/BP_Storage.UpdateValue` _storage2 (+ ValueToAdd (`/Game/Blueprints/BP_Storage.CurrentVolume` _storage2))))

(fn `EmptyTanks`
  (returns (TanksVolume :type "Float (double-precision)"))
  (locals (Volume :type "Float (double-precision)"))
  (set `local.Volume` (`/Game/Blueprints/BP_Storage.CurrentVolume` (`self.Storage1`)))
  (`/Game/Blueprints/BP_Storage.UpdateValue` (`self.Storage1`) 0.0)
  (`/Game/Blueprints/BP_Storage.UpdateValue` (`self.Storage2`) 0.0)
  (return (`local.Volume`)))

(fn `UserConstructionScript`)