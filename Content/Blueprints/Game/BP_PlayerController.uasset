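; Player controller for the rover pawn, translating input into movement, mining and game restarts.
; On BeginPlay it caches the BP_GameMode and controlled BP_Rover references.
; Movement axes drive the rover along its cine camera's forward and right vectors, projected onto the ground plane and normalized for camera-relative, horizontal motion.
; Interact calls the rover's Mine, and RestartGame restarts only while the game mode is waiting for a restart.
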(event `self.ReceiveBeginPlay`
  (bind _asbp_game_mode (cast `/Game/Blueprints/Game/BP_GameMode` (`GameplayStatics.GetGameMode`)))
  (set `self.GameMode` _asbp_game_mode)
  (bind _asbp_rover (cast `/Game/Blueprints/Characters/BP_Rover` (`self.K2_GetPawn`)))
  (set `self.Rover` _asbp_rover))

(event `InputAxis|MoveUpDown`
  (params (AxisValue :type "Float (single-precision)"))
  (bind _rover (`self.Rover`))
  (`/Engine/EditorBlueprintResources/StandardMacros.IsValid` _rover
    (:`Is Valid`
      (`Pawn.AddMovementInput` _rover (* AxisValue (`self.GetAbsoluteForward`)) 1.0 false))))

(event `InputAxis|MoveRigthLeft`
  (params (AxisValue :type "Float (single-precision)"))
  (bind _rover (`self.Rover`))
  (`/Engine/EditorBlueprintResources/StandardMacros.IsValid` _rover
    (:`Is Valid`
      (`Pawn.AddMovementInput` _rover (* AxisValue (`self.GetAbsoluteRight`)) 1.0 false))))

(event `InputAction|Interact`
  (params (Key :type "Key Structure"))
  (bind _rover (`self.Rover`))
  (:`Pressed`
    (`/Engine/EditorBlueprintResources/StandardMacros.IsValid` _rover
      (:`Is Valid`
        (`/Game/Blueprints/Characters/BP_Rover.Mine` _rover)))))

(event `InputAction|RestartGame`
  (params (Key :type "Key Structure"))
  (:`Pressed`
    (if (`/Game/Blueprints/Game/BP_GameMode.IsWaitingForRestart` (`self.GameMode`))
      (`/Game/Blueprints/Game/BP_GameMode.Restart` (`self.GameMode`)))))

(fn `GetAbsoluteForward`
  (returns (AbsoluteForward :type "Vector Structure"))
  (return (`KismetMathLibrary.Normal` (`KismetMathLibrary.ProjectVectorOnToPlane` (`SceneComponent.GetForwardVector` (`/Game/Blueprints/Characters/BP_Rover.CineCamera` (`self.Rover`))) (0.0 0.0 1.0)))))

(fn `GetAbsoluteRight`
  (returns (AbsoluteRigth :type "Vector Structure"))
  (return (`KismetMathLibrary.Normal` (`KismetMathLibrary.ProjectVectorOnToPlane` (`SceneComponent.GetRightVector` (`/Game/Blueprints/Characters/BP_Rover.CineCamera` (`self.Rover`))) (0.0 0.0 1.0)))))

(fn `UserConstructionScript`)