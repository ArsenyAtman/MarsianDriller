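; Game mode that handles the game-over and restart flow around the base's fuel supply.
; On BeginPlay it finds the first BP_Base and binds GameOver to its out-of-fuel event.
; GameOver sets the waiting-for-restart flag and destroys every BP_Alien in the level.
; A separate Restart event, not triggered within this graph, opens the Mars level.
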(event `self.ReceiveBeginPlay`
  (bind _outactors (`GameplayStatics.GetAllActorsOfClass` "/Game/Blueprints/Gameplay/BP_Base.BP_Base_C"))
  (bind _output_get (set `self.Base` (`|GetArrayItem` _outactors)))
  (add `/Game/Blueprints/Gameplay/BP_Base.OnRunnedOutOfFuel` _output_get (delegate `GameOver`)))

(event `GameOver`
  (set `self.IsWaitingForRestart` true)
  (bind _outactors (`GameplayStatics.GetAllActorsOfClass` "/Game/Blueprints/Characters/BP_Alien.BP_Alien_C"))
  (for _array_element _outactors
    (`self.K2_DestroyActor` _array_element)))

(event `Restart`
  (`GameplayStatics.OpenLevelBySoftObjectPtr` "/Game/Maps/Mars.Mars"))

(fn `UserConstructionScript`)