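; BP_Storage is a storage Blueprint that displays its current volume as the height of a cylinder.
; UpdateValue clamps the new volume between zero and Capacity, then scales the cylinder's height by the fill ratio times VerticalScale, keeping SideScale for its width.
; It also raises the cylinder in proportion to that height, so the fill grows upward from a fixed base.
; The construction script calls UpdateValue to show the starting volume.
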(event `UpdateValue`
  (params (NewValue :type "Float (double-precision)"))
  (bind _cylinder (`self.Cylinder`))
  (bind _sidescale (`self.SideScale`))
  (bind _returnvalue (* (/ (`self.CurrentVolume`) (`self.Capacity`)) (`self.VerticalScale`)))
  (set `self.CurrentVolume` (`KismetMathLibrary.FClamp` NewValue 0.0 (`self.Capacity`)))
  (`SceneComponent.K2_SetRelativeLocation` _cylinder (`KismetMathLibrary.MakeVector` 0.0 0.0 (* 50.0 _returnvalue)) false false)
  (`SceneComponent.SetRelativeScale3D` _cylinder (`KismetMathLibrary.MakeVector` _sidescale _sidescale _returnvalue)))

(fn `UserConstructionScript`
  (`self.UpdateValue` (`self.CurrentVolume`)))