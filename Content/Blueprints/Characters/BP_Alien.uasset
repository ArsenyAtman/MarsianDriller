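; BP_Alien is an alien character that makes periodic vocal sounds and can attack a rover.
; From BeginPlay, Talk plays its audio and re-arms a one-shot timer with a random delay, forming an endless chatter loop.
; Attack sends the target Rover an interact message, fires the OnAttack dispatcher and plays an impact sound.
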(event `self.ReceiveBeginPlay`
  (`self.Talk`))

(event `Talk`
  (`AudioComponent.Play` (`self.TalkAudio`) 0.0)
  (`KismetSystemLibrary.K2_SetTimerDelegate` (delegate `Talk`) (`KismetMathLibrary.RandomFloatInRange` (`self.TalkDelayMin`) (`self.TalkDelayMax`))))

(event `Attack`
  (params (Rover :type "/Game/Blueprints/Characters/BP_Rover Object Reference"))
  (message `/Game/Blueprints/Gameplay/BPI_Interactable.Interact` Rover self)
  (`self.OnAttack`)
  (`AudioComponent.Play` (`self.ImpactAudio`) 0.0))

(fn `UserConstructionScript`)