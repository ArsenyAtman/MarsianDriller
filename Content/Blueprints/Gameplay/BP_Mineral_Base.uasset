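; Base Blueprint for a harvestable mineral that a rover interacts with to fill its tanks by a random amount.
; Collecting sets it not ready and starts a one-shot timer with a random delay that restores it.
; A ready flag gates interaction, and a scale timeline grows the mesh on restore and reverses to shrink it on collection.
; Minerals that begin play not ready start that restore timer immediately.
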(event `self.ReceiveBeginPlay`
  (if (not (`self.bIsReady`))
    (`self.StartRestore`)))

(event `StartRestore`
  (`KismetSystemLibrary.K2_SetTimerDelegate` (delegate `Restore`) (`KismetMathLibrary.RandomFloatInRange` (`self.RestoreTimeMin`) (`self.RestoreTimeMax`))))

(event `Restore`
  (`self.UpdateCondition` true))

(event `Collect`
  (if (`self.bIsReady`)
    (`self.UpdateCondition` false)
    (`self.StartRestore`)))

(event `UpdateCondition`
  (params (bReady :type Boolean))
  (bind _output_get (set `self.bIsReady` bReady))
  (if _output_get
    (bind (_direction _scale) (`Timeline|ScaleTimeline` :!label _label)
      (:`Update`
        (`SceneComponent.SetWorldScale3D` (`self.Mesh`) (`KismetMathLibrary.MakeVector` _scale _scale _scale))))
    (else
      (goto _label :!via `ReverseFromEnd`))))

(event `/Game/Blueprints/Gameplay/BPI_Interactable.Interact`
  (params (Interactor :type "Pawn Object Reference"))
  (if (`self.bIsReady`)
    (bind _asbp_rover (cast `/Game/Blueprints/Characters/BP_Rover` Interactor))
    (`/Game/Blueprints/Characters/BP_Rover.FillTanks` _asbp_rover (`KismetMathLibrary.RandomFloatInRange` (`self.RestoreValueMin`) (`self.RestoreValueMax`)))
    (`self.Collect`)))

(fn `UserConstructionScript`)