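; BP_Base is a base actor that burns fuel over time and gets refuelled by the rover.
; It takes its BP_Storage from the FuelStorage child actor on BeginPlay and lowers that volume every tick at FuelConsumptionSpeed.
; When the volume equals zero it fires the OnRunnedOutOfFuel event.
; Interacting with a BP_Rover empties the rover's tanks into the storage.
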(event `self.ReceiveBeginPlay`
  (bind _asbp_storage (cast `/Game/Blueprints/Gameplay/BP_Storage` (`ChildActorComponent.ChildActor` (`self.FuelStorage`))))
  (set `self.Storage` _asbp_storage))

(event `self.ReceiveTick`
  (params (DeltaSeconds :type "Float (single-precision)"))
  (`/Game/Blueprints/Gameplay/BP_Storage.UpdateValue` (`self.Storage`) (- (`/Game/Blueprints/Gameplay/BP_Storage.CurrentVolume` (`self.Storage`)) (* DeltaSeconds (`self.FuelConsumptionSpeed`))))
  (if (== (`/Game/Blueprints/Gameplay/BP_Storage.CurrentVolume` (`self.Storage`)) 0.0)
    (`self.OnRunnedOutOfFuel`)))

(event `/Game/Blueprints/Gameplay/BPI_Interactable.Interact`
  (params (Interactor :type "Pawn Object Reference"))
  (bind _storage (`self.Storage`))
  (bind _asbp_rover (cast `/Game/Blueprints/Characters/BP_Rover` Interactor))
  (bind _tanksvolume (`/Game/Blueprints/Characters/BP_Rover.EmptyTanks` _asbp_rover))
  (`/Game/Blueprints/Gameplay/BP_Storage.UpdateValue` _storage (+ _tanksvolume (`/Game/Blueprints/Gameplay/BP_Storage.CurrentVolume` _storage))))

(fn `UserConstructionScript`)